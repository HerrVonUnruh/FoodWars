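; UnitSpawner is a Blueprint that automatically places units on the combat grid when play begins.
; After a delay it spawns one unit at a hard-coded tile, then switches UnitType and, after another delay, spawns two more.
; ExecuteAction spawns a BP_Unit and registers it with the CombatSystem through PlayerActions.
; Its valid-tile check does not affect spawning, and logic to remove an occupying unit is disconnected.
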(event `self.ReceiveBeginPlay`
  (`KismetSystemLibrary.Delay` 3.0)
  (set `self.UnitType` "NewEnumerator4")
  (`self.Execute Action` (make `IntPoint` 1 12))
  (set `self.UnitType` "NewEnumerator0")
  (`KismetSystemLibrary.Delay` 3.0)
  (`self.Execute Action` (make `IntPoint` 1 11))
  (`self.Execute Action` (make `IntPoint` 1 13)))

(fn `Execute Action`
  (params (Index :type "IntPoint Structure"))
  (bind _unitdata (`/Game/Robin/NewLevel/Blueprint/Core/Units/Utilities/BFL_Units.GetDefaultUnitDataFromUnitType` (`self.UnitType`)))
  (if (`KismetArrayLibrary.Array_Contains` (break `/Game/Robin/NewLevel/Blueprint/Core/Units/Utilities/S_UnitData_Stats` (`.Stats_8_763C327A4C9BFE567B3B0A803DB7CA30` (break `/Game/Robin/NewLevel/Blueprint/Core/Units/Utilities/S_UnitData` _unitdata))) (`.Type_6_271F7E2B4AFF42C0F984C1861E1BDC31` (break `/Game/Robin/NewLevel/Blueprint/Grid/Utilities/S_TileData` (`BlueprintMapLibrary.Map_Find` (`/Game/Robin/NewLevel/Blueprint/Grid/BP_Grid.GridTiles` (`/Game/Robin/NewLevel/Blueprint/Core/Player/BP_PlayerActions.Grid` (`self.PlayerActions`))) (`local.Index`)))))
    _
    (else
      _))
  (bind _returnvalue (`|SpawnActorFromClass` "/Game/Robin/NewLevel/Blueprint/Core/Units/BP_Unit.BP_Unit_C" (`KismetMathLibrary.MakeTransform` (0.0 0.0 0.0)) "AlwaysSpawn" "OverrideRootScale" null (`self.UnitType`) null))
  (`/Game/Robin/NewLevel/Blueprint/Core/Combat/BP_CombatSystem.AddUnitInCombat` (`/Game/Robin/NewLevel/Blueprint/Core/Player/BP_PlayerActions.CombatSystem` (`self.PlayerActions`)) _returnvalue (`local.Index`)))

(fn `UserConstructionScript`
  (`parent.UserConstructionScript`))