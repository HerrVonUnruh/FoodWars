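; BP_PC is the player script that handles Space-bar rolls of a universal (red) and pawn (blue) die with a cup (Becher).
; RollDice triggers both dice, rotates the cup, then after a fixed delay takes each die's highest side component and parses its value from the component's name.
; Separately, the key handler polls until both dice stop moving, then briefly shows the stored results in WP_DiceRoll, independently of that delay.
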(event `self.ReceiveBeginPlay`
  (bind _dice_wp_ref (`self.Dice_WP_Ref`))
  (set `self.bShowMouseCursor` true)
  (bind _outactors (`GameplayStatics.GetAllActorsOfClass` "/Game/Development/Blueprints/BP_Universal_Dice.BP_Universal_Dice_C"))
  (set `self.universalDiceRef` (`|GetArrayItem` _outactors))
  (bind _outactors_2 (`GameplayStatics.GetAllActorsOfClass` "/Game/Development/Blueprints/BP_Pawn_Dice.BP_Pawn_Dice_C"))
  (set `self.pDiceRef` (`|GetArrayItem` _outactors_2))
  (bind _outactors_3 (`GameplayStatics.GetAllActorsOfClass` "/Game/Development/Blueprints/BP_Becher.BP_Becher_C"))
  (set `self.BecherRef` (`|GetArrayItem` _outactors_3))
  (bind _returnvalue (`|CreateWidget` "/Game/Development/UI/WP_DiceRoll.WP_DiceRoll_C"))
  (bind _output_get (set `self.Dice_WP_Ref` _returnvalue))
  (`UserWidget.AddToViewport` _output_get 0)
  (set `self.WP Universal Dice` (`/Game/Development/UI/WP_DiceRoll.WP_Universal_Dice` _dice_wp_ref))
  (set `self.WP Pawn Dice` (`/Game/Development/UI/WP_DiceRoll.WP_Pawn_Dice` _dice_wp_ref)))

(event `Roll Dice`
  (bind _universaldiceref (`self.universalDiceRef`))
  (bind _pdiceref (`self.pDiceRef`))
  (`/Engine/EditorBlueprintResources/StandardMacros.DoOnce` false :!label _label
    (:`Completed`
      (set `self.CanRoll` false)
      (`/Game/Development/Blueprints/BP_Pawn_Dice.Roll Pawn Dice` _pdiceref)
      (`/Game/Development/Blueprints/BP_Universal_Dice.Roll Universal Dice` _universaldiceref)
      ;[0.1915 1 0.255] Becher
      (`self.K2_SetActorRotation` (`self.BecherRef`) (struct :`Pitch` -180.0) false)
      (`KismetSystemLibrary.Delay` 5.0)
      (set `self.uHighest_ZAxis` 10.0)
      (set `self.pHighest_ZAxis` 10.0)
      (for _array_element (`/Game/Development/Blueprints/BP_Universal_Dice.uSideArr` _universaldiceref)
        (bind (_returnvalue_x _returnvalue_y _returnvalue_z) (`KismetMathLibrary.BreakVector` (`SceneComponent.K2_GetComponentLocation` _array_element)))
        (if (< (`self.uHighest_ZAxis`) _returnvalue_z)
          (set `self.uHighest_ZAxis` _returnvalue_z)
          (bind _output_get (set `self.uTempStaticMesh` _array_element))))
      (for _array_element_2 (`/Game/Development/Blueprints/BP_Pawn_Dice.pSideArr` _pdiceref)
        (bind (_returnvalue_x_2 _returnvalue_y_2 _returnvalue_z_2) (`KismetMathLibrary.BreakVector` (`SceneComponent.K2_GetComponentLocation` _array_element_2)))
        (if (< (`self.pHighest_ZAxis`) _returnvalue_z_2)
          (set `self.pHighest_ZAxis` _returnvalue_z_2)
          (bind _output_get_2 (set `self.pTempStaticMesh` _array_element_2))))
      (bind _returnvalue (`KismetStringLibrary.GetCharacterAsNumber` (`KismetSystemLibrary.GetDisplayName` _output_get) 18))
      ;[1 0 0 1 72] Universal/Red Dice
      (if (== _returnvalue 49)
        (set `self.ResultUniversalDice` 1)
        (set `self.E_Universal_Dice_Results` "NewEnumerator0")
        (bind _returnvalue_2 (`KismetStringLibrary.GetCharacterAsNumber` (`KismetSystemLibrary.GetDisplayName` _output_get_2) 13))
        ;[0 0.07026 1 1 72] Pawn/BlueDice
        (if (== _returnvalue_2 49) :!label _label_2
          (set `self.ResultPawnDice` 1)
          (set `self.E_Pawn_Dice_Results` "NewEnumerator0")
          (set `self.CanRoll` true :!label _label_3)
          (goto _label :!via `Reset`)
          (elif (== _returnvalue_2 50)
            (set `self.ResultPawnDice` 2)
            (set `self.E_Pawn_Dice_Results` "NewEnumerator1")
            (goto _label_3)
            (elif (== _returnvalue_2 51)
              (set `self.ResultPawnDice` 3)
              (set `self.E_Pawn_Dice_Results` "NewEnumerator2")
              (goto _label_3)
              (elif (== _returnvalue_2 52)
                (set `self.ResultPawnDice` 4)
                (set `self.E_Pawn_Dice_Results` "NewEnumerator3")
                (goto _label_3)
                (elif (== _returnvalue_2 53)
                  (set `self.ResultPawnDice` 5)
                  (set `self.E_Pawn_Dice_Results` "NewEnumerator4")
                  (goto _label_3)
                  (elif (== _returnvalue_2 54)
                    (set `self.ResultPawnDice` 6)
                    (set `self.E_Pawn_Dice_Results` "NewEnumerator5")
                    (goto _label_3)))))))
        (elif (== _returnvalue 50)
          (set `self.ResultUniversalDice` 2)
          (set `self.E_Universal_Dice_Results` "NewEnumerator1")
          (goto _label_2)
          (elif (== _returnvalue 51)
            (set `self.ResultUniversalDice` 3)
            (set `self.E_Universal_Dice_Results` "NewEnumerator2")
            (goto _label_2)
            (elif (== _returnvalue 52)
              (set `self.ResultUniversalDice` 4)
              (set `self.E_Universal_Dice_Results` "NewEnumerator3")
              (goto _label_2)
              (elif (== _returnvalue 53)
                (set `self.ResultUniversalDice` 5)
                (set `self.E_Universal_Dice_Results` "NewEnumerator4")
                (goto _label_2)
                (elif (== _returnvalue 54)
                  (set `self.ResultUniversalDice` 6)
                  (set `self.E_Universal_Dice_Results` "NewEnumerator5")
                  (goto _label_2))))))))))

(event `Key|SpaceBar`
  (params (Key :type "Key Structure"))
  (bind _dice_wp_ref (`self.Dice_WP_Ref`))
  (bind _returnvalue (`self.K2_GetActorLocation` (`self.universalDiceRef`)))
  (bind _returnvalue_2 (`self.K2_GetActorLocation` (`self.pDiceRef`)))
  (:`Pressed`
    (if (`self.CanRoll`)
      (`self.Roll Dice`)
      (set `self.uDiceLocation` _returnvalue_2 :!label _label_4)
      (set `self.pDiceLocation` _returnvalue)
      (`KismetSystemLibrary.Delay` 1.0)
      (if (and (== (`self.uDiceLocation`) _returnvalue_2) (== (`self.pDiceLocation`) _returnvalue))
        (`Widget.SetVisibility` (`self.Dice_WP_Ref`) "Visible")
        (`|ExecutionSequence`
          (:`then_0`
            (switch `/Game/Development/Blueprints/E_Universal_Dice_Results` (`self.E_Universal_Dice_Results`)
              (:`NewEnumerator0`
                (`/Game/Development/UI/WP_DiceRoll.Display_Universal_Dice_Roll` _dice_wp_ref "/Game/Art/YannickConceptsDice1.YannickConceptsDice1"))
              (:`NewEnumerator1`
                (`/Game/Development/UI/WP_DiceRoll.Display_Universal_Dice_Roll` _dice_wp_ref "/Game/Art/YannickConceptsDice2.YannickConceptsDice2"))
              (:`NewEnumerator2`
                (`/Game/Development/UI/WP_DiceRoll.Display_Universal_Dice_Roll` _dice_wp_ref "/Game/Art/YannickConceptsDice3.YannickConceptsDice3"))
              (:`NewEnumerator3`
                (`/Game/Development/UI/WP_DiceRoll.Display_Universal_Dice_Roll` _dice_wp_ref "/Game/Art/YannickConceptsDice4.YannickConceptsDice4"))
              (:`NewEnumerator4`
                (`/Game/Development/UI/WP_DiceRoll.Display_Universal_Dice_Roll` _dice_wp_ref "/Game/Art/YannickConceptsDice5.YannickConceptsDice5"))
              (:`NewEnumerator5`
                (`/Game/Development/UI/WP_DiceRoll.Display_Universal_Dice_Roll` _dice_wp_ref "/Game/Art/YannickConceptsDice6.YannickConceptsDice6"))))
          (:`then_1`
            (switch `/Game/Development/Blueprints/E_Pawn_Dice_Results` (`self.E_Pawn_Dice_Results`)
              (:`NewEnumerator0`
                (`/Game/Development/UI/WP_DiceRoll.Display_Pawn_Dice_Roll` _dice_wp_ref "/Game/Art/YannickConceptsDice1.YannickConceptsDice1"))
              (:`NewEnumerator1`
                (`/Game/Development/UI/WP_DiceRoll.Display_Pawn_Dice_Roll` _dice_wp_ref "/Game/Art/YannickConceptsDice2.YannickConceptsDice2"))
              (:`NewEnumerator2`
                (`/Game/Development/UI/WP_DiceRoll.Display_Pawn_Dice_Roll` _dice_wp_ref "/Game/Art/YannickConceptsDice3.YannickConceptsDice3"))
              (:`NewEnumerator3`
                (`/Game/Development/UI/WP_DiceRoll.Display_Pawn_Dice_Roll` _dice_wp_ref "/Game/Art/YannickConceptsDice4.YannickConceptsDice4"))
              (:`NewEnumerator4`
                (`/Game/Development/UI/WP_DiceRoll.Display_Pawn_Dice_Roll` _dice_wp_ref "/Game/Art/YannickConceptsDice5.YannickConceptsDice5"))
              (:`NewEnumerator5`
                (`/Game/Development/UI/WP_DiceRoll.Display_Pawn_Dice_Roll` _dice_wp_ref "/Game/Art/YannickConceptsDice6.YannickConceptsDice6")))))
        (`KismetSystemLibrary.Delay` 2.0)
        (`Widget.SetVisibility` _dice_wp_ref "Collapsed")
        (else
          (goto _label_4))))))

(fn `UserConstructionScript`)