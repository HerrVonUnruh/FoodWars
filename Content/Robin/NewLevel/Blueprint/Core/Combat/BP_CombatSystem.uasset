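; BP_CombatSystem tracks the units in combat and keeps their grid indices, tile occupancy and world positions in sync.
; Adding a unit hands it the Grid and listens for it reaching new tiles; removal uses a sentinel off-grid index and optionally destroys the actor.
; When the grid regenerates or a tile changes, affected units are re-placed, or removed and destroyed if the tile type is invalid for them.
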(event `self.ReceiveBeginPlay`
  (bind _grid (`self.Grid`))
  (add `/Game/Robin/NewLevel/Blueprint/Grid/BP_Grid.OnGridGenerated` _grid (`|CreateDelegate` :!event `OnGridGenerated`))
  (add `/Game/Robin/NewLevel/Blueprint/Grid/BP_Grid.OnTileDataUpdated` _grid (`|CreateDelegate` :!event `OnTileDataUpdatet`)))

(fn `AddUnitInCombat`
  (params (Unit :type "/Game/Robin/NewLevel/Blueprint/Core/Units/BP_Unit Object Reference") (Index :type "IntPoint Structure"))
  (`KismetArrayLibrary.Array_Add` (`self.UnitsInCombat`) (`local.Unit`))
  (`self.SetUnitIndexOnGrid` (`local.Unit`) (`local.Index`))
  (`/Game/Robin/NewLevel/Blueprint/Core/Units/BP_Unit.SetGrid` (`local.Unit`) (`self.Grid`))
  (add `/Game/Robin/NewLevel/Blueprint/Core/Units/BP_Unit.OnUnitReachNewTile` (`local.Unit`) (`|CreateDelegate` :!event `OnUnitReachedNewTile`)))

(fn `OnGridGenerated`
  (locals (CopyOfUnitsInCombat :type "Array of /Game/Robin/NewLevel/Blueprint/Core/Units/BP_Unit Object Reference"))
  (bind _output_get (set `local.CopyOfUnitsInCombat` (`self.UnitsInCombat`)))
  (for _array_element _output_get
    (bind _index (`/Game/Robin/NewLevel/Blueprint/Core/Units/BP_Unit.Index` _array_element))
    (if (`KismetArrayLibrary.Array_Contains` (break `/Game/Robin/NewLevel/Blueprint/Core/Units/Utilities/S_UnitData_Stats` (`.Stats_8_763C327A4C9BFE567B3B0A803DB7CA30` (break `/Game/Robin/NewLevel/Blueprint/Core/Units/Utilities/S_UnitData` (`/Game/Robin/NewLevel/Blueprint/Core/Units/BP_Unit.UnitData` _array_element)))) (`.Type_6_271F7E2B4AFF42C0F984C1861E1BDC31` (break `/Game/Robin/NewLevel/Blueprint/Grid/Utilities/S_TileData` (`BlueprintMapLibrary.Map_Find` (`/Game/Robin/NewLevel/Blueprint/Grid/BP_Grid.GridTiles` (`self.Grid`)) _index))))
      (`self.SetUnitIndexOnGrid` _array_element _index true)
      (else
        (`self.RemoveUnitFromCombat` _array_element)))))

(fn `OnTileDataUpdatet`
  (params (Index :type "IntPoint Structure"))
  (locals (CopyOfUnitsInCombat :type "Array of /Game/Robin/NewLevel/Blueprint/Core/Units/BP_Unit Object Reference"))
  (bind _output_get (set `local.CopyOfUnitsInCombat` (`self.UnitsInCombat`)))
  (for _array_element _output_get
    (bind _index (`/Game/Robin/NewLevel/Blueprint/Core/Units/BP_Unit.Index` _array_element))
    (if (`KismetMathLibrary.Equal_IntPointIntPoint` (`local.Index`) _index)
      (if (`KismetArrayLibrary.Array_Contains` (break `/Game/Robin/NewLevel/Blueprint/Core/Units/Utilities/S_UnitData_Stats` (`.Stats_8_763C327A4C9BFE567B3B0A803DB7CA30` (break `/Game/Robin/NewLevel/Blueprint/Core/Units/Utilities/S_UnitData` (`/Game/Robin/NewLevel/Blueprint/Core/Units/BP_Unit.UnitData` _array_element)))) (`.Type_6_271F7E2B4AFF42C0F984C1861E1BDC31` (break `/Game/Robin/NewLevel/Blueprint/Grid/Utilities/S_TileData` (`BlueprintMapLibrary.Map_Find` (`/Game/Robin/NewLevel/Blueprint/Grid/BP_Grid.GridTiles` (`self.Grid`))))))
        (`self.SetUnitIndexOnGrid` _array_element _index)
        (break)
        (else
          (`self.RemoveUnitFromCombat` _array_element)
          (break))))))

(fn `OnUnitReachedNewTile`
  (params (Unit :type "/Game/Robin/NewLevel/Blueprint/Core/Units/BP_Unit Object Reference") (Index :type "IntPoint Structure"))
  (`self.SetUnitIndexOnGrid` Unit Index))

(fn `RemoveUnitFromCombat`
  (params (Unit :type "/Game/Robin/NewLevel/Blueprint/Core/Units/BP_Unit Object Reference") (DestroyActor :type Boolean :default true))
  (`KismetArrayLibrary.Array_RemoveItem` (`self.UnitsInCombat`) (`local.Unit`))
  (`self.SetUnitIndexOnGrid` (`local.Unit`) (make `IntPoint` -999 -999))
  (if DestroyActor
    (`self.K2_DestroyActor` (`local.Unit`))))

(fn `SetUnitIndexOnGrid`
  (params (Unit :type "/Game/Robin/NewLevel/Blueprint/Core/Units/BP_Unit Object Reference") (Index :type "IntPoint Structure") (Force :type Boolean :default false))
  (locals (`Previous Tile` :type "/Game/Robin/NewLevel/Blueprint/Grid/Utilities/S_TileData Structure"))
  (bind (_value _returnvalue) (`BlueprintMapLibrary.Map_Find` (`/Game/Robin/NewLevel/Blueprint/Grid/BP_Grid.GridTiles` (`self.Grid`)) (`local.Index`)))
  (bind _transform_location (`KismetMathLibrary.BreakTransform` (break `/Game/Robin/NewLevel/Blueprint/Grid/Utilities/S_TileData` _value)))
  (`|ExecutionSequence`
    (:`then_0`
      (if (or (!= (`/Game/Robin/NewLevel/Blueprint/Core/Units/BP_Unit.Index` (`local.Unit`)) (`local.Index`)) (`local.Force`))
        (`|ExecutionSequence`
          (:`then_0`
            (bind _output_get (set `local.Previous Tile` (`BlueprintMapLibrary.Map_Find` (`/Game/Robin/NewLevel/Blueprint/Grid/BP_Grid.GridTiles` (`self.Grid`)) (`/Game/Robin/NewLevel/Blueprint/Core/Units/BP_Unit.Index` (`local.Unit`)))))
            (if (== (`.UnitOnTile_15_46C1785F43DE82D2A681E6BD5E1D4E53` (break `/Game/Robin/NewLevel/Blueprint/Grid/Utilities/S_TileData` _output_get)) (`local.Unit`))
              (bind _structout (setmembers `/Game/Robin/NewLevel/Blueprint/Grid/Utilities/S_TileData` :`StructRef` (`local.Previous Tile`) :`UnitOnTile` null))
              (`BlueprintMapLibrary.Map_Add` (`/Game/Robin/NewLevel/Blueprint/Grid/BP_Grid.GridTiles` (`self.Grid`)) (`.Index_4_04F06BC449CAA02AB06B81A8F6A005BB` (break `/Game/Robin/NewLevel/Blueprint/Grid/Utilities/S_TileData` _structout)) _structout)))
          (:`then_1`
            (set `/Game/Robin/NewLevel/Blueprint/Core/Units/BP_Unit.Index` (`local.Index`) (`local.Unit`))
            (if (!= (`local.Index`) (make `IntPoint` -999 -999))
              (bind _structout_2 (setmembers `/Game/Robin/NewLevel/Blueprint/Grid/Utilities/S_TileData` :`StructRef` (`BlueprintMapLibrary.Map_Find` (`/Game/Robin/NewLevel/Blueprint/Grid/BP_Grid.GridTiles` (`self.Grid`)) (`local.Index`)) :`UnitOnTile` (`local.Unit`)))
              (`BlueprintMapLibrary.Map_Add` (`/Game/Robin/NewLevel/Blueprint/Grid/BP_Grid.GridTiles` (`self.Grid`)) (`.Index_4_04F06BC449CAA02AB06B81A8F6A005BB` (break `/Game/Robin/NewLevel/Blueprint/Grid/Utilities/S_TileData` _structout_2)) _structout_2)))
          (:`then_2`
            (`self.OnUnitGridIndexChanged` (`local.Unit`))))))
    (:`then_1`
      (`self.K2_SetActorLocation` (`local.Unit`) (select `bool` _returnvalue :`false` (-99999.0 -99999.0 -99999.0) :`true` _transform_location) false false))))

(fn `UserConstructionScript`)