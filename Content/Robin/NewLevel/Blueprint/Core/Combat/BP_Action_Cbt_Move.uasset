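; Combat move action for a grid-based battle that marks the tiles the selected unit can reach.
; On BeginPlay it binds to the grid's reachables pathfinder and, when the unit differs from the cached one, clears the old tile state.
; It then runs a delayed, frame-budgeted search using the unit's movement points, diagonal rule and valid tile types.
; The completion handler applies the tile state to each reachable index.
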(event `self.ReceiveBeginPlay`
  (`parent.ReceiveBeginPlay`)
  (add `/Game/Robin/NewLevel/Blueprint/Grid/BP_GridPathfinding.OnPathfindingCompleted` (`/Game/Robin/NewLevel/Blueprint/Grid/BP_Grid.GridPathfinding_Reachables` (`/Game/Robin/NewLevel/Blueprint/Core/Player/BP_PlayerActions.Grid` (`self.PlayerActions`))) (`|CreateDelegate` :!event `OnPathfindingCompletedReachables`))
  (`self.GenerateReachable` (`/Game/Robin/NewLevel/Blueprint/Core/Player/BP_PlayerActions.SelectedUnit` (`self.PlayerActions`))))

(fn `GenerateReachable`
  (params (Unit :type "/Game/Robin/NewLevel/Blueprint/Core/Units/BP_Unit Object Reference"))
  (bind _currentunitforreachables (`self.CurrentUnitForReachables`))
  (bind (_validtiletypes _canmovediagonally _mp_pawn) (break `/Game/Robin/NewLevel/Blueprint/Core/Units/Utilities/S_UnitData_Stats` (`.Stats_8_763C327A4C9BFE567B3B0A803DB7CA30` (break `/Game/Robin/NewLevel/Blueprint/Core/Units/Utilities/S_UnitData` (`/Game/Robin/NewLevel/Blueprint/Core/Units/BP_Unit.UnitData` _currentunitforreachables)))))
  (if (!= Unit (`self.CurrentUnitForReachables`))
    (set `self.CurrentUnitForReachables` Unit)
    (`/Game/Robin/NewLevel/Blueprint/Grid/BP_Grid.ClearStateFromTiles` (`/Game/Robin/NewLevel/Blueprint/Core/Player/BP_PlayerActions.Grid` (`self.PlayerActions`)) "NewEnumerator7")
    (`/Game/Robin/NewLevel/Blueprint/Grid/BP_GridPathfinding.FindPath` (`/Game/Robin/NewLevel/Blueprint/Grid/BP_Grid.GridPathfinding_Reachables` (`/Game/Robin/NewLevel/Blueprint/Core/Player/BP_PlayerActions.Grid` (`self.PlayerActions`))) (`/Game/Robin/NewLevel/Blueprint/Core/Units/BP_Unit.Index` _currentunitforreachables) (make `IntPoint` -999 -999) _canmovediagonally _validtiletypes 0.1 15.0 true _mp_pawn)))

(fn `OnPathfindingCompletedReachables`
  (params (Reachables :type "Array of IntPoint Structure"))
  (for _array_element Reachables
    (`/Game/Robin/NewLevel/Blueprint/Grid/BP_Grid.AddStateToTile` (`/Game/Robin/NewLevel/Blueprint/Core/Player/BP_PlayerActions.Grid` (`self.PlayerActions`)) _array_element "NewEnumerator7")))

(fn `UserConstructionScript`
  (`parent.UserConstructionScript`))