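; Spell animation actor for the Run Chicken spell, showing an animated chicken icon on the target tile in combat.
; On play, it moves to the target tile and sets the Run Chicken texture on its widget component's image.
; A timeline drives the widget's height, draw size and opacity, then signals spell animation completion when finished.
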(event `self.Event_PlaySpellAnimation`
  (bind _widget (`self.Widget`))
  (bind _transform_location (`KismetMathLibrary.BreakTransform` (`self.GetTileTransform` (`self.TargetIndex`))))
  (`self.K2_SetActorLocation` _transform_location)
  (bind _output_get (set `self.W_Image` (cast `/Game/Robin/NewLevel/Blueprint/Core/CombatSetup/Spells/SpellAnimations/W_Image` (`WidgetComponent.GetUserWidgetObject` (`self.Widget`)) :!pure true)))
  (`Image.SetBrushFromTexture` (`/Game/Robin/NewLevel/Blueprint/Core/CombatSetup/Spells/SpellAnimations/W_Image.Image_Component` _output_get) "/Game/Robin/NewLevel/Blueprint/Core/CombatSetup/Spells/SpellAnimations/Assets/Icon_RunChickenRun_NoBackground.Icon_RunChickenRun_NoBackground" false)
  (bind (_direction _locationz _drawsize _opacity) (`Timeline|Timeline_RunChicken`)
    (:`Update`
      (`SceneComponent.K2_SetRelativeLocation` _widget (`KismetMathLibrary.MakeVector` 0.0 0.0 _locationz) false false)
      (`WidgetComponent.SetDrawSize` _widget (`KismetMathLibrary.MakeVector2D` _drawsize _drawsize))
      (`Widget.SetRenderOpacity` (`self.W_Image`) _opacity))
    (:`Finished`
      (`self.Event_CompleteSpellAnimation`))))

(fn `UserConstructionScript`
  (`parent.UserConstructionScript`))