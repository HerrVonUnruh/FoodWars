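; BP_AnimatedShape is an actor in the combat spell components that displays a colored static mesh animated between two transforms.
; On BeginPlay it applies its Mesh, Material and Color variables to the AnimatedShape mesh component, passing the color as a material vector parameter.
; A Timeline then drives an alpha that interpolates the whole actor's transform from OriginTransform to TargetTransform.
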(event `self.ReceiveBeginPlay`
  (bind _animatedshape (`self.AnimatedShape`))
  (`StaticMeshComponent.SetStaticMesh` _animatedshape (`self.Mesh`))
  (`PrimitiveComponent.SetMaterial` _animatedshape 0 (`self.Material`))
  (`MeshComponent.SetVectorParameterValueOnMaterials` _animatedshape "Color" (`KismetMathLibrary.Conv_LinearColorToVector` (`self.Color`)))
  (bind (_direction _transformalpha) (`Timeline|Timeline` :!via `PlayFromStart`)
    (:`Update`
      (`self.K2_SetActorTransform` (`KismetMathLibrary.TLerp` (`self.OriginTransform`) (`self.TargetTransform`) _transformalpha)))))

(fn `UserConstructionScript`)