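; BP_GridModifier is an editor-placed marker that assigns a tile type, such as obstacle, higher movement cost or flying-only, to part of a grid.
; Its construction script takes the mesh and flat material for the chosen grid shape and tints it by type as a filled color preview.
; It overlaps a custom trace channel, presumably so the grid can detect it, and stays hidden in game.
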(fn `UserConstructionScript`
  (bind _staticmesh (`self.StaticMesh`))
  (bind (_data_meshsize _data_mesh _data_meshmaterial _data_flatmesh _data_flatmaterial) (break `/Game/Robin/NewLevel/Blueprint/Grid/Gridshapes/S_GridShapeData` (`/Game/Robin/NewLevel/Blueprint/Grid/Gridshapes/BFL_GridShape.Get Shape Data` (`self.Shape`))))
  (`StaticMeshComponent.SetStaticMesh` _staticmesh _data_mesh)
  (`PrimitiveComponent.SetMaterial` _staticmesh 0 _data_flatmaterial)
  (`MeshComponent.SetVectorParameterValueOnMaterials` _staticmesh "Color" (`KismetMathLibrary.Conv_LinearColorToVector` (select `/Game/Robin/NewLevel/Blueprint/Grid/Utilities/E_TileType` (`self.Type`) :`NewEnumerator1` (struct :`R` 1.0 :`G` 1.0 :`B` 1.0 :`A` 1.0) :`NewEnumerator2` (struct :`R` 0.820833 :`A` 1.0) :`NewEnumerator3` (struct :`R` 0.166466 :`G` 0.660954 :`B` 0.7375 :`A` 1.0) :`NewEnumerator4` (struct :`R` 0.05146 :`G` 0.055385 :`B` 0.295833 :`A` 1.0) :`NewEnumerator5` (struct :`R` 0.836391 :`G` 0.85 :`B` 0.0425 :`A` 1.0) :!type "LinearColor Structure")))
  (`MeshComponent.SetScalarParameterValueOnMaterials` _staticmesh "IsFilled" 1.0)
  (`PrimitiveComponent.SetCollisionResponseToChannel` (`self.StaticMesh`) "ECC_GameTraceChannel3" "ECR_Overlap")
  (`self.SetActorHiddenInGame` true))