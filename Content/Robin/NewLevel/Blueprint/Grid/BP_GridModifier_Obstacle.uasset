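; BP_GridModifier_Obstacle is a grid modifier actor shown in the editor as a colored tile shape and hidden in game.
; Its construction script takes the mesh and flat material from the Shape's data, then colors it filled according to Type, which covers obstacles, special tiles and team colors.
; It overlaps one custom trace channel and blocks another, and has no active event logic.
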(fn `UserConstructionScript`
  (bind _staticmesh (`self.StaticMesh`))
  (bind _staticmesh_2 (`self.StaticMesh`))
  (bind (_data_meshsize _data_mesh _data_meshmaterial _data_flatmesh _data_flatmaterial) (break `/Game/Robin/NewLevel/Blueprint/Grid/Gridshapes/S_GridShapeData` (`/Game/Robin/NewLevel/Blueprint/Grid/Gridshapes/BFL_GridShape.Get Shape Data` (`self.Shape`))))
  (`StaticMeshComponent.SetStaticMesh` _staticmesh _data_mesh)
  (`PrimitiveComponent.SetMaterial` _staticmesh 0 _data_flatmaterial)
  (`MeshComponent.SetVectorParameterValueOnMaterials` _staticmesh "Color" (`KismetMathLibrary.Conv_LinearColorToVector` (select `/Game/Robin/NewLevel/Blueprint/Grid/Utilities/E_TileType` (`self.Type`) :`NewEnumerator1` (struct :`R` 1.0 :`G` 1.0 :`B` 1.0 :`A` 1.0) :`NewEnumerator2` (struct :`R` 0.820833 :`A` 1.0) :`NewEnumerator3` (struct :`R` 0.166466 :`G` 0.660954 :`B` 0.7375 :`A` 1.0) :`NewEnumerator4` (struct :`R` 0.05146 :`G` 0.055385 :`B` 0.295833 :`A` 1.0) :`NewEnumerator5` (struct :`R` 0.836391 :`G` 0.85 :`B` 0.0425 :`A` 1.0) :`NewEnumerator6` (struct :`R` 0.007556 :`G` 0.375 :`A` 1.0) :`NewEnumerator7` (struct :`R` 0.333333 :`B` 0.043629 :`A` 1.0) :`NewEnumerator8` (struct :`G` 0.054063 :`B` 0.291667 :`A` 1.0) :`NewEnumerator9` (struct :`R` 0.28125 :`G` 0.2495 :`A` 1.0) :`NewEnumerator10` (struct :`R` 1.0 :`G` 0.431106 :`A` 1.0) :!type "LinearColor Structure")))
  (`MeshComponent.SetScalarParameterValueOnMaterials` _staticmesh "IsFilled" 1.0)
  (`PrimitiveComponent.SetCollisionResponseToChannel` _staticmesh_2 "ECC_GameTraceChannel1" "ECR_Overlap")
  (`PrimitiveComponent.SetCollisionResponseToChannel` _staticmesh_2 "ECC_GameTraceChannel4" "ECR_Block")
  (`self.SetActorHiddenInGame` true))