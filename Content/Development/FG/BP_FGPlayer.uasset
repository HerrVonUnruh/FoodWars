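; BP_FGPlayer is a fighting-game prototype player that moves a Sphere component when the Punch input is pressed.
; BeginPlay caches the first FightCharacter in the level, whose move direction scales Dir into the punch's Y offset.
; MoveComponentTo drives the move while a ButtonPressed flag pauses Tick.
; Otherwise, Tick resets the sphere's relative location from the actor's world location, shifted back on X.
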(event `self.ReceiveBeginPlay`
  (bind _outactors (`GameplayStatics.GetAllActorsOfClass` "/Script/FoodWars.FightCharacter"))
  (set `self.fightRef` (`|GetArrayItem` _outactors)))

(event `self.ReceiveActorBeginOverlap`
  (params (OtherActor :type "Actor Object Reference")))

(event `self.ReceiveTick`
  (params (DeltaSeconds :type "Float (single-precision)"))
  (bind (_returnvalue_x _returnvalue_y _returnvalue_z) (`KismetMathLibrary.BreakVector` (`self.K2_GetActorLocation`)))
  (if (not (`self.button pressed`))
    (`SceneComponent.K2_SetRelativeLocation` (`self.Sphere`) (`KismetMathLibrary.MakeVector` (+ _returnvalue_x -100.0) _returnvalue_y _returnvalue_z) false false)))

(event `InputAction|InputAction_Punch`
  (params (Key :type "Key Structure"))
  (:`Pressed`
    (set `self.button pressed` true)
    (bind _returnvalue (`FightCharacter.getMoveDir` (`self.fightRef`)))
    (`KismetSystemLibrary.MoveComponentTo` (`self.Sphere`) (+ (`SceneComponent.K2_GetComponentLocation` (`self.Sphere`)) (`KismetMathLibrary.MakeVector` 0.0 (* (`self.dir`) _returnvalue))))
    (set `self.button pressed` false)))

(fn `UserConstructionScript`)