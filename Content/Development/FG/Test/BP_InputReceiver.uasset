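; BP_InputReceiver is a test per-player input receiver that turns a Start press into a request to the game mode.
; With a valid character select reference, it asks the game mode to spawn the player, passing its player index and itself, then prints a debug "Hello".
; Otherwise it asks the game mode to display character select for that player index.
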(event `InputAction|Start`
  (params (Key :type "Key Structure"))
  (:`Pressed`
    (if (`KismetSystemLibrary.IsValid` (`self.characterSelectRef`))
      (message `/Game/Development/FG/Test/TEST_IFG.Spawn Player` (`GameplayStatics.GetGameMode`) (`self.PlayerIndex`) self)
      (`KismetSystemLibrary.PrintString` "Hello")
      (else
        (message `/Game/Development/FG/Test/TEST_IFG.DisplayCharacterSelecet` (`GameplayStatics.GetGameMode`) (`self.PlayerIndex`))))))

(event `InputAction|MoveRightInWidget`
  (params (Key :type "Key Structure")))

(event `InputAction|MoveLeftInWidget`
  (params (Key :type "Key Structure")))

(fn `UserConstructionScript`)