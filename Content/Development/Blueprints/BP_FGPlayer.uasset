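; BP_FGPlayer is a player Blueprint that prototypes a punch by moving a Sphere component.
; Each Tick, while ButtonPressed is false, it places the Sphere at the actor's location offset along X.
; The Punch input sets the flag, lunges the Sphere along Y with a short MoveComponentTo, then clears the flag.
; Both paths feed world-space positions into relative-location inputs.
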(event `self.ReceiveActorBeginOverlap`
  (params (OtherActor :type "Actor Object Reference")))

(event `self.ReceiveTick`
  (params (DeltaSeconds :type "Float (single-precision)"))
  (bind (_returnvalue_x _returnvalue_y _returnvalue_z) (`KismetMathLibrary.BreakVector` (`self.K2_GetActorLocation`)))
  (if (not (`self.button pressed`))
    (`SceneComponent.K2_SetRelativeLocation` (`self.Sphere`) (`KismetMathLibrary.MakeVector` (+ _returnvalue_x -100.0) _returnvalue_y _returnvalue_z) false false)))

(event `InputAction|InputAction_Punch`
  (params (Key :type "Key Structure"))
  (:`Pressed`
    (set `self.button pressed` true)
    (`KismetSystemLibrary.MoveComponentTo` (`self.Sphere`) (+ (`SceneComponent.K2_GetComponentLocation` (`self.Sphere`)) (0.0 300.0 0.0)) (struct) false false 0.2)
    (set `self.button pressed` false)))

(fn `UserConstructionScript`)