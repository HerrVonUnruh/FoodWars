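; BP_Pawn_Dice is a six-sided physics die that is thrown when RollPawnDice is called.
; A roll randomizes the actor's rotation, moves it to a fixed raised drop point and applies a large random angular impulse to the Dice component.
; BeginPlay collects the six Side references into SideArr, though this graph never reads the result.
; A random linear impulse is present but unconnected.
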(event `self.ReceiveBeginPlay`
  (set `self.sideArr` (`|MakeArray` (`self.Side 1`) (`self.Side 2`) (`self.Side 3`) (`self.Side 4`) (`self.Side 5`) (`self.Side 6`))))

(event `Roll Pawn Dice`
  (`self.K2_SetActorRotation` (`KismetMathLibrary.MakeRotator` (`KismetMathLibrary.RandomFloatInRange` -180.0 180.0) (`KismetMathLibrary.RandomFloatInRange` -180.0 180.0) (`KismetMathLibrary.RandomFloatInRange` -180.0 180.0)))
  (`self.K2_SetActorLocation` (130.0 0.0 1000.0))
  (`PrimitiveComponent.AddAngularImpulseInDegrees` (`self.dice`) (`KismetMathLibrary.MakeVector` (`KismetMathLibrary.RandomFloatInRange` 1000000.0 2000000.0) (`KismetMathLibrary.RandomFloatInRange` 1000000.0 2000000.0) (`KismetMathLibrary.RandomFloatInRange` 1000000.0 2000000.0)) "None" false))

(fn `UserConstructionScript`)